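; Central controller for a card-scanner user and sales app that reads card UUIDs from an Arduino over serial and swaps UI screens.
; On startup it loads file-based settings, opens Home and optionally connects.
; A delayed polling loop routes new cards to Show User or Add User based on whether a UUID save file exists.
; Rescanning the same card briefly raises a flag that a second loop uses to confirm pending sales.
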(event Custom|MainLoop
  (params (Active :type Boolean))
  (|MainLoopGraph Active))

(event Custom|CardConfirm
  (|ConfirmCardGraph))

(event Custom|CheckForCardConfirm
  (params (Active :type Boolean))
  (|CheckForCardConfirmGraph Active))

(event EventBeginPlay
  (|StartupGraph))

(event EventEndPlay
  (params (EndPlayReason :type EEndPlayReason%20Enum :default "Destroyed"))
  (CallFunction|Disconnect))

(fn ConstructionScript)

(fn CreateWidget
  (params (PageToOpen :type Enum_Pages%20Enum :default "NewEnumerator0"))
  (switch Utilities|FlowControl|Switch|SwitchonEnum_Pages PageToOpen
    (:NewEnumerator0
      (|HomeScreenGraph))
    (:NewEnumerator1
      (|AddUserGraph))
    (:NewEnumerator2
      (|ShowUserGraph))
    (:NewEnumerator3
      (|MakeSalesGraph))
    (:NewEnumerator5
      (|EditUserGraph))
    (:NewEnumerator6
      (|HomeScreenGraph_2))))

(fn CloseOpenWidget
  (params (WidgetTarget :type Widget%20Object%20Reference) (PageToOpen :type Enum_Pages%20Enum :default "NewEnumerator0"))
  (Widget|SetIsEnabled WidgetTarget false)
  (Widget|RemovefromParent WidgetTarget)
  (Utilities|Platform|CollectGarbage)
  (CallFunction|CreateWidget PageToOpen))

(fn Disconnect
  (bind _arduinoref (Variables|Refrences|GetArduinoRef))
  (Utilities|IsValid _arduinoref
    (:Is%20Valid
      (if (Class|Serial|IsOpened _arduinoref)
        (Class|Serial|Close _arduinoref)
        (if (Variables|Settings|Debug|GetDebugActive)
          (Development|PrintString (Utilities|String|ToString(Text) (Utilities|Text|FormatText "PORT {#} CLOSED SUCCESSFULLY" (Variables|Settings|GetSerialPortToConnectTo))) true true "(R=0.000000,G=1.000000,B=0.000000,A=1.000000)" (Variables|Settings|Debug|GetDebugMessageTime)))
        (elif (Variables|Settings|Debug|GetDebugActive)
          (Development|PrintString "UNABLE TO DISCONNECT FROM SERIAL 
SERIAL PORT WAS NOT CURRENTLY OPEN" true true "(R=1.000000,G=1.000000,B=0.000000,A=1.000000)" (Variables|Settings|Debug|GetDebugMessageTime)))))
    (:Is%20Not%20Valid
      (if (Variables|Settings|Debug|GetDebugActive)
        (Development|PrintString "UNABLE TO DISCONNECT FROM SERIAL 
ARDUINO REFRENCE WAS NOT VALID 
WAS THE CONNECTION SUCCESSFUL?" true true "(R=1.000000,G=1.000000,B=0.000000,A=1.000000)" (Variables|Settings|Debug|GetDebugMessageTime))))))

(fn Connect
  (params (Port :type Integer))
  (bind (_bopened _returnvalue) (Class|Serial|OpenComPort Port 9600))
  (if _bopened
    (if (Variables|Settings|Debug|GetDebugActive)
      (Development|PrintString (Utilities|String|ToString(Text) (Utilities|Text|FormatText "SUCCESSFULLY CONNECTED TO SERIAL PORT {#}" (Variables|Settings|GetSerialPortToConnectTo))) true true "(R=0.000000,G=1.000000,B=0.000000,A=1.000000)" (Variables|Settings|Debug|GetDebugMessageTime)))
    (Variables|Refrences|SetArduinoRef _returnvalue)
    (CallFunction|MainLoop true)
    (return true)
    (else
      (if (Variables|Settings|Debug|GetDebugActive)
        (Development|PrintString "UNABLE TO CONNECT TO SERIAL PORT REQUESTED " true true "(R=1.000000,G=0.000000,B=0.000000,A=1.000000)" (Variables|Settings|Debug|GetDebugMessageTime)))
      (return false))))

(fn ClearLastUUID
  (Variables|Runtime(Don'tEdit)|SetLast_UUID_Scanned ""))

(fn LoadSettings
  (bind _returnvalue (Class|BlueprintPathsLibrary|ProjectSavedDir))
  (bind (_report _success _stringinfile) (Class|SSZFileFunctions|LoadStringfromFile _returnvalue "Settings.SSZ" :!label _label))
  (if _success
    (Variables|Settings|SetSerialPortToConnectTo (Math|Conversions|ToInteger(Byte) (Utilities|Array|Get(acopy) (Utilities|SchemaRowDecoder _stringinfile))))
    (Variables|Settings|Debug|SetDebugActive (Utilities|StringtoBool (Utilities|Array|Get(acopy) (Utilities|SchemaRowDecoder _stringinfile) 1)))
    (Variables|Settings|SetShouldConnectOnStart (Utilities|StringtoBool (Utilities|Array|Get(acopy) (Utilities|SchemaRowDecoder _stringinfile) 2)))
    (else
      (Class|SSZFileFunctions|SaveStringtoFile _returnvalue "Settings.SSZ" (Utilities|SchemaRowEncoder (Utilities|Array|MakeArray (Utilities|String|ToString(Integer) (Variables|Settings|GetSerialPortToConnectTo)) (Utilities|String|ToString(Boolean) (Variables|Settings|Debug|GetDebugActive)) (Utilities|String|ToString(Boolean) (Variables|Settings|GetShouldConnectOnStart)))) false)
      (goto _label))))

(fn SaveSettings
  (Class|SSZFileFunctions|SaveStringtoFile (Class|BlueprintPathsLibrary|ProjectSavedDir) "Settings.SSZ" (Utilities|SchemaRowEncoder (Utilities|Array|MakeArray (Utilities|String|ToString(Integer) (Variables|Settings|GetSerialPortToConnectTo)) (Utilities|String|ToString(Boolean) (Variables|Settings|Debug|GetDebugActive)) (Utilities|String|ToString(Boolean) (Variables|Settings|GetShouldConnectOnStart)))) true))